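; BP_carretera is a road zone actor that speeds up BP_agent characters while they overlap it.
; On begin overlap it multiplies the agent's CharacterMovement MaxWalkSpeed by 1.5, and on end overlap it scales it back by the reciprocal.
; The change is relative to the current speed rather than stored, so overlapping several of these actors stacks the boost.
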(event `self.ReceiveActorBeginOverlap`
  (params (OtherActor :type "Actor Object Reference"))
  (bind _asbp_agent (cast `/Game/MINE/blueprints/BP_agent` OtherActor))
  (bind _charactermovement (`Character.CharacterMovement` _asbp_agent))
  (set `CharacterMovementComponent.MaxWalkSpeed` (* (`CharacterMovementComponent.MaxWalkSpeed` _charactermovement) 1.5) _charactermovement))

(event `self.ReceiveActorEndOverlap`
  (params (OtherActor :type "Actor Object Reference"))
  (bind _asbp_agent (cast `/Game/MINE/blueprints/BP_agent` OtherActor))
  (bind _charactermovement (`Character.CharacterMovement` _asbp_agent))
  (set `CharacterMovementComponent.MaxWalkSpeed` (* (`CharacterMovementComponent.MaxWalkSpeed` _charactermovement) 0.666667) _charactermovement))

(fn `UserConstructionScript`)