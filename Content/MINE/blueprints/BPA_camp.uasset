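; Camp building actor that endlessly spawns actors of a configurable class belonging to its faction.
; BeginPlay runs a loop that waits a random few seconds, then spawns the class at a fixed world-axis offset from the camp, passing on its Faccion.
; The Construction Script creates a dynamic roof-tile material instance on the static mesh and tints it with the faction's color.
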(event `self.ReceiveBeginPlay`
  (`parent.ReceiveBeginPlay`)
  (`KismetSystemLibrary.Delay` (`KismetMathLibrary.RandomFloatInRange` 5.0 10.0) :!label _label)
  (`|SpawnActorFromClass` (`self.classToGenerate`) (`KismetMathLibrary.MakeTransform` (+ (.location (`self.GetTransform`)) (300.0 0.0 50.0)) (.rotation (`self.GetTransform`)) (.scale (`self.GetTransform`))) "Undefined" "MultiplyWithRoot" null (`self.faccion`) null)
  (goto _label))

(fn `UserConstructionScript`
  (`parent.UserConstructionScript`)
  (bind _returnvalue (`PrimitiveComponent.CreateDynamicMaterialInstance` (`self.StaticMesh`) 2 "/Game/Fantastic_Village_Pack/materials/MI_rooftiles_01.MI_rooftiles_01" "None"))
  (`MaterialInstanceDynamic.SetVectorParameterValue` _returnvalue "Base Color Tint" (`/Game/MINE/blueprints/BPL_faccion.getColorFaccion` (`self.faccion`))))