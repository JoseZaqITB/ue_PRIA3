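; BP_agent is an actor with a Health value that displays it on a text component and dies when that health runs out.
; Each tick it writes Health to the Texter and rotates that text from the player pawn's rotation plus a fixed offset so it faces the viewer.
; AnyDamage subtracts incoming damage from Health and destroys the actor at zero or below.
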(event `self.ReceiveTick`
  (params (DeltaSeconds :type "Float (single-precision)"))
  (bind _texter (`self.texter`))
  ;[1 1 1] colocar la salud del actor en su texter
  (`TextRenderComponent.K2_SetText` _texter (`KismetTextLibrary.Conv_DoubleToText` (`self.health`) "HalfToEven"))
  ;[1 1 1] colocar el texto viendo a la camara
  (`SceneComponent.K2_SetWorldRotation` _texter (`KismetMathLibrary.ComposeRotators` (`self.K2_GetActorRotation` (`GameplayStatics.GetPlayerPawn` 0)) (struct :`Pitch` 90.0 :`Yaw` 180.0)) false false))

(event `self.ReceiveAnyDamage`
  (params (Damage :type "Float (single-precision)") (DamageType :type "DamageType Object Reference") (InstigatedBy :type "Controller Object Reference") (DamageCauser :type "Actor Object Reference"))
  ;[1 1 1] restar salud
  (bind _output_get (set `self.health` (- (`self.health`) Damage)))
  ;[1 1 1] matar jugador si <= 0 su salud
  (if (<= _output_get 0.0)
    (`self.K2_DestroyActor`)))

(fn `UserConstructionScript`)