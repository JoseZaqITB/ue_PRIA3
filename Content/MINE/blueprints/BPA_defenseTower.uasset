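; BPA_defenseTower is an AI-controlled defense watchtower pawn, tinted to the color of its faction.
; When possessed by an AI controller, it runs the BT_towerDefense behavior tree, which holds its behavior.
; The construction script puts a dynamic wood-plank material instance on the watchtower mesh and sets its base color tint from Faccion.
; BeginPlay only calls the parent, and Tick is disabled.
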(event `self.ReceiveBeginPlay`
  (`parent.ReceiveBeginPlay`))

(event `self.ReceivePossessed`
  (params (NewController :type "Controller Object Reference"))
  ;[1 1 1] Añadimos un comportamiento de tipo Behavior tree a la IA
  (bind _asaicontroller (cast `AIController` NewController))
  (`AIController.RunBehaviorTree` _asaicontroller "/Game/MINE/AI/BT_towerDefense.BT_towerDefense"))

(fn `UserConstructionScript`
  (`parent.UserConstructionScript`)
  (bind _returnvalue (`PrimitiveComponent.CreateDynamicMaterialInstance` (`self.SM_PROP_watchtower_wood_01`) 1 "/Game/Fantastic_Village_Pack/materials/MI_wood_planks_05.MI_wood_planks_05" "None"))
  (`MaterialInstanceDynamic.SetVectorParameterValue` _returnvalue "Base Color Tint" (`/Game/MINE/blueprints/BPL_faccion.getColorFaccion` (`self.faccion`))))