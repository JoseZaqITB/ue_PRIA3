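; BP_bomb is a faction-aware bomb that damages nearby enemy BP_agent pawns when something overlaps its Box.
; The overlap runs a sphere query of radius DamageRatio, then applies Damage and spawns sparks on each agent of another Faction.
; A Delay inside the loop precedes emitter deactivation and setting Exploited, so the post-loop destroy check runs before that delayed flag is set.
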(event `self.Box.OnComponentBeginOverlap`
  (params (OverlappedComponent :type "PrimitiveComponent Object Reference") (OtherActor :type "Actor Object Reference") (OtherComp :type "PrimitiveComponent Object Reference") (OtherBodyIndex :type Integer) (bFromSweep :type Boolean) (SweepResult :type "HitResult Structure (by ref)"))
  ;[1 1 1] proyecta una esfera donde recoge todos los actores dentro
  (bind _outactors (`KismetSystemLibrary.SphereOverlapActors` (`self.K2_GetActorLocation`) (`self.damageRatio`) (`|MakeArray` "ObjectTypeQuery3" :!type "EObjectTypeQuery Enum")))
  (for _array_element _outactors
    ;[1 1 1] verificar que es un enemigo
    (bind _asbp_agent (cast `/Game/MINE/blueprints/BP_agent` _array_element))
    (if (`|EnumInequality` (`/Game/MINE/blueprints/BP_agent.faccion` _asbp_agent) (`self.faccion`))
      ;[1 1 1] crea un efecto de particula y ataca. Espera cierto tiempo pa vovler a atacas. La ejecucion acaba con exito despues de atacar
      (bind _returnvalue (`GameplayStatics.SpawnEmitterAtLocation` "/Game/Realistic_Starter_VFX_Pack_Vol2/Particles/Sparks/P_Sparks_G.P_Sparks_G" (`self.K2_GetActorLocation` _asbp_agent) (struct) (1.0 1.0 1.0) true "ManualRelease"))
      (`GameplayStatics.ApplyDamage` _asbp_agent (`self.damage`))
      ;;[1 1 1] desactivar el looping de la particula
      (`KismetSystemLibrary.Delay` 0.5)
      (`ActorComponent.Deactivate` _returnvalue)
      (set `self.exploited` true)))
  ;[1 1 1] si llegó a explotar, destruir el actor
  (if (`self.exploited`)
    (`self.K2_DestroyActor`)))

(fn `UserConstructionScript`)