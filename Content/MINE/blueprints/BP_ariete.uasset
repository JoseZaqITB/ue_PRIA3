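; BP_ariete is an AI-controlled battering ram pawn that belongs to either the Red or Blue faction.
; On BeginPlay it switches on Faccion and toggles the visibility of one of its two flag meshes, setting the banner color for its side.
; When possessed by an AIController, it runs the BT_ariete behavior tree, leaving all further behavior to that tree.
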(event `self.ReceiveBeginPlay`
  ;[1 1 1] coloca el color de la bandera segun la faccion
  (switch `/Game/MINE/blueprints/ENUM_faccion` (`self.faccion`)
    (:`NewEnumerator0`
      (`SceneComponent.ToggleVisibility` (`self.SM_PROP_flag_06`) false))
    (:`NewEnumerator1`
      (`SceneComponent.ToggleVisibility` (`self.SM_PROP_flag_05_blue`) false))))

(event `self.ReceivePossessed`
  (params (NewController :type "Controller Object Reference"))
  ;[1 1 1] Añadimos un comportamiento de tipo Behavior tree a la IA
  (bind _asaicontroller (cast `AIController` NewController))
  (`AIController.RunBehaviorTree` _asaicontroller "/Game/MINE/AI/BT_ariete.BT_ariete"))

(fn `UserConstructionScript`
  (`parent.UserConstructionScript`))