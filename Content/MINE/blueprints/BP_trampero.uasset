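; BP_trampero is an AI character, a trapper by its name, whose body color reflects its faction.
; When possessed by an AI controller, it runs the BT_trampero behavior tree.
; The construction script creates a dynamic instance of MI_Manny_02 on the mesh and sets its Tint from the faction via the GetColorFaccion library function.
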(event `self.ReceivePossessed`
  (params (NewController :type "Controller Object Reference"))
  ;[1 1 1] Añadimos un comportamiento de tipo Behavior tree a la IA
  (bind _asaicontroller (cast `AIController` NewController))
  (`AIController.RunBehaviorTree` _asaicontroller "/Game/MINE/AI/BT_trampero.BT_trampero"))

(fn `UserConstructionScript`
  (`parent.UserConstructionScript`)
  ;[1 1 1] cambiar el color del personaje segun su faccion. Se utiliza la funcion de BPL_faccion para determinar su color
  (bind _returnvalue (`PrimitiveComponent.CreateDynamicMaterialInstance` (`self.Mesh`) 0 "/Game/Characters/Mannequins/Materials/Instances/Manny/MI_Manny_02.MI_Manny_02" "None"))
  (`MaterialInstanceDynamic.SetVectorParameterValue` _returnvalue "Tint" (`/Game/MINE/blueprints/BPL_faccion.getColorFaccion` (`self.faccion`))))